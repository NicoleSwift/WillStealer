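; Player controller for a game where a parasite possesses cultists, also setting up cursor widgets and music.
; Tick rotates the pawn's ArrowGun toward the cursor hit and updates the parasite's tentacle flipbook through CheckIsPossessable.
; That check box-traces ahead for an unstunned, unmasked cultist facing away, whom IA_Action then possesses.
; Hotkeys handle time-dilation pause, level restart, and save, load and score debugging via the game instance.
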(event Input|EnhancedActionEvents|EnhancedInputActionIA_Action
  (params (ActionValue :type Boolean) (ElapsedSeconds :type Float%20%28double-precision%29) (TriggeredSeconds :type Float%20%28double-precision%29) (InputAction :type Input%20Action%20Object%20Reference :default "/Game/Inputs/IA_Action.IA_Action"))
  (bind (_pawn_to_possess _is_possesable_) (CallFunction|CheckIsPossessable?))
  (if _is_possesable_
    (Utilities|IsValid _pawn_to_possess
      (:Is%20Valid
        (Pawn|Possess _pawn_to_possess)
        (Audio|PlaySound2D "/Game/Sounds/SND_Possessing.SND_Possessing" 1.0 1.0 0.0 0 0)
        (Audio|PlaySound2D "/Game/Sounds/GRWL_ROAR_ANGRY.GRWL_ROAR_ANGRY" 1.0 1.0 0.0 0 0)))))

(event EventBeginPlay
  (Variables|BP_PlayerController_C|SetPaused? self false)
  (Input|SetInputModeGameandUI self 0 "DoNotLock" false true)
  (bind _returnvalue (UserInterface|CreateWidget "/Game/Widgets/Cursor_Crosshair.Cursor_Crosshair_C"))
  (Class|PlayerController|SetMouseCursorWidget "Crosshairs" _returnvalue)
  (bind _returnvalue_2 (UserInterface|CreateWidget "/Game/Widgets/Cursor_Default.Cursor_Default_C"))
  (Class|PlayerController|SetMouseCursorWidget "Default" _returnvalue_2)
  (Audio|PlaySound2D "/Game/Sounds/Creepy_80_s_Horror_Theme_-_Bad_Omen_⧸⧸_Royalty_Free_No_Copyright_Music.Creepy_80_s_Horror_Theme_-_Bad_Omen_⧸⧸_Royalty_Free_No_Copyright_Music" 0.25 1.0 0.0 0 0))

(event EventTick
  (params (DeltaSeconds :type Float%20%28single-precision%29))
  (bind (_hitresult _returnvalue) (Game|Player|GetHitResultUnderCursorbyChannel "TraceTypeQuery3" true))
  (bind _location (Collision|BreakHitResult _hitresult))
  (if (not (Variables|Default|GetPaused?))
    (bind _asbp_characters_parent (Utilities|Casting|CastToBP_Characters_Parent (Pawn|GetControlledPawn)))
    (if _returnvalue
      (Transformation|SetWorldRotation (Variables|/Game/Blueprints/BP_Characters_Parent.BP_Characters_Parent_C|GetArrow_Gun _asbp_characters_parent) (Math|Rotator|MakeRotator 2.7e+02 (.pitch (Math|Rotator|FindLookatRotation (Math|Vector|MakeVector (.x (Transformation|GetWorldLocation (Variables|/Game/Blueprints/BP_Characters_Parent.BP_Characters_Parent_C|GetArrow_Gun _asbp_characters_parent))) (.y (Transformation|GetWorldLocation (Variables|/Game/Blueprints/BP_Characters_Parent.BP_Characters_Parent_C|GetArrow_Gun _asbp_characters_parent))) 0.0) (Math|Vector|MakeVector (.x _location) (.y _location) 0.0))) (.yaw (Math|Rotator|FindLookatRotation (Math|Vector|MakeVector (.x (Transformation|GetWorldLocation (Variables|/Game/Blueprints/BP_Characters_Parent.BP_Characters_Parent_C|GetArrow_Gun _asbp_characters_parent))) (.y (Transformation|GetWorldLocation (Variables|/Game/Blueprints/BP_Characters_Parent.BP_Characters_Parent_C|GetArrow_Gun _asbp_characters_parent))) 0.0) (Math|Vector|MakeVector (.x _location) (.y _location) 0.0)))) false false)
      (bind _asbp_parasite (Utilities|Casting|CastToBP_Parasite (Pawn|GetControlledPawn)))
      (Sprite|SetFlipbook (Variables|/Game/Blueprints/BP_Characters_Parent.BP_Characters_Parent_C|GetGun_FlipBook _asbp_parasite) "/Game/Flipbooks/FB_Tentacle_Idle.FB_Tentacle_Idle")
      (CallFunction|CheckIsPossessable?))))

(event Input|KeyboardEvents|P
  (params (Key :type Key%20Structure :default "None"))
  (:Pressed
    (Utilities|FlowControl|FlipFlop
      (:A
        (Utilities|Time|SetGlobalTimeDilation 0.0)
        (Variables|Default|SetPaused? true))
      (:B
        (Utilities|Time|SetGlobalTimeDilation 1.0)
        (Variables|Default|SetPaused? false)))))

(event Input|KeyboardEvents|1
  (params (Key :type Key%20Structure :default "None"))
  ;[1 1 1] Comment
  (:Pressed
    (Default|SaveGame (.AsWS%20Game%20Instance (Utilities|Casting|CastToWS_Game_Instance (Game|GetGameInstance))))))

(event Input|KeyboardEvents|R
  (params (Key :type Key%20Structure :default "None"))
  ;[1 1 1] Comment
  (:Pressed
    (bind _returnvalue (Game|GetCurrentLevelName true))
    (Game|OpenLevel(byName) (Utilities|String|StringToName _returnvalue))))

(event Input|KeyboardEvents|2
  (params (Key :type Key%20Structure :default "None"))
  ;[1 1 1] Comment
  (:Pressed
    (Default|LoadGame (.AsWS%20Game%20Instance (Utilities|Casting|CastToWS_Game_Instance (Game|GetGameInstance))))))

(event Input|KeyboardEvents|3
  (params (Key :type Key%20Structure :default "None"))
  (bind _returnvalue (Game|GetGameInstance))
  (bind _asws_game_instance (Utilities|Casting|CastToWS_Game_Instance _returnvalue))
  (bind _saved_game_ref (Variables|/Game/Blueprints/WS_Game_Instance.WS_Game_Instance_C|GetSaved_Game_Ref _asws_game_instance))
  ;[1 1 1] Comment
  (:Pressed
    (Variables|/Game/Blueprints/WS_Save_Game.WS_Save_Game_C|SetScore _saved_game_ref (+ (Variables|/Game/Blueprints/WS_Save_Game.WS_Save_Game_C|GetScore _saved_game_ref) 1))
    (Development|PrintString (Utilities|String|ToString(Integer) (Variables|/Game/Blueprints/WS_Save_Game.WS_Save_Game_C|GetScore _saved_game_ref)))))

(event Input|KeyboardEvents|4
  (params (Key :type Key%20Structure :default "None"))
  (bind _returnvalue (Game|GetGameInstance))
  (bind _asws_game_instance (Utilities|Casting|CastToWS_Game_Instance _returnvalue))
  (bind _saved_game_ref (Variables|/Game/Blueprints/WS_Game_Instance.WS_Game_Instance_C|GetSaved_Game_Ref _asws_game_instance))
  ;[1 1 1] Comment
  (:Pressed
    (Variables|/Game/Blueprints/WS_Save_Game.WS_Save_Game_C|SetScore _saved_game_ref (- (Variables|/Game/Blueprints/WS_Save_Game.WS_Save_Game_C|GetScore _saved_game_ref) 1))
    (Development|PrintString (Utilities|String|ToString(Integer) (Variables|/Game/Blueprints/WS_Save_Game.WS_Save_Game_C|GetScore _saved_game_ref)))))

(event Input|KeyboardEvents|5
  (params (Key :type Key%20Structure :default "None"))
  ;[1 1 1] Comment
  (:Pressed
    (Development|PrintString (Utilities|String|ToString(Integer) (Variables|/Game/Blueprints/WS_Save_Game.WS_Save_Game_C|GetScore (Variables|/Game/Blueprints/WS_Game_Instance.WS_Game_Instance_C|GetSaved_Game_Ref (.AsWS%20Game%20Instance (Utilities|Casting|CastToWS_Game_Instance (Game|GetGameInstance)))))))))

(fn ConstructionScript)

(fn CheckIsPossessable?
  (bind _asbp_characters_parent (Utilities|Casting|CastToBP_Characters_Parent (Pawn|GetControlledPawn)))
  (bind _outhit (Collision|BoxTraceByChannel (Transformation|GetWorldLocation (Variables|/Game/Blueprints/BP_Characters_Parent.BP_Characters_Parent_C|GetArrow_Gun _asbp_characters_parent)) (+ (Transformation|GetWorldLocation (Variables|/Game/Blueprints/BP_Characters_Parent.BP_Characters_Parent_C|GetArrow_Gun _asbp_characters_parent)) (* (Math|Vector|GetForwardVector (Variables|/Game/Blueprints/BP_Characters_Parent.BP_Characters_Parent_C|GetArrow_Gun _asbp_characters_parent)) 5e+01)) "20.000000,20.000000,10.000000" "0, 0, 0" "TraceTypeQuery2" false (Utilities|Array|MakeArray (Pawn|GetControlledPawn)) "None"))
  (bind _aspawn (Utilities|Casting|CastToPawn (.HitActor (Collision|BreakHitResult _outhit))))
  (bind _asbp_cultist_parent (Utilities|Casting|CastToBP_Cultist_Parent _aspawn))
  (if (Math|Boolean|ANDBoolean (> (Math|Vector|DotProduct (Math|Vector|Normalize (- (Transformation|GetActorLocation _aspawn) (Transformation|GetActorLocation (Pawn|GetControlledPawn)))) (Math|Vector|GetForwardVector (Variables|/Script/Engine.Actor|GetRootComponent _aspawn))) 0.1) (not (ScalableFloat|GetValueasBool (AI|GetBlackboard (.AsBP%20Enemy%20Controller (Utilities|Casting|CastToBP_Enemy_Controller (Pawn|GetController _aspawn)))) (Utilities|Name|MakeLiteralName "is Stanned?"))) (not (Variables|/Game/Blueprints/BP_Cultist_Parent.BP_Cultist_Parent_C|GetProtected_By_Mask? _asbp_cultist_parent)))
    (bind _asbp_parasite (Utilities|Casting|CastToBP_Parasite (Pawn|GetControlledPawn)))
    (Sprite|SetFlipbook (Variables|/Game/Blueprints/BP_Characters_Parent.BP_Characters_Parent_C|GetGun_FlipBook _asbp_parasite) "/Game/Flipbooks/FB_Tentacle_Ready.FB_Tentacle_Ready")
    (return _aspawn (Math|Boolean|ANDBoolean (> (Math|Vector|DotProduct (Math|Vector|Normalize (- (Transformation|GetActorLocation _aspawn) (Transformation|GetActorLocation (Pawn|GetControlledPawn)))) (Math|Vector|GetForwardVector (Variables|/Script/Engine.Actor|GetRootComponent _aspawn))) 0.1) (not (ScalableFloat|GetValueasBool (AI|GetBlackboard (.AsBP%20Enemy%20Controller (Utilities|Casting|CastToBP_Enemy_Controller (Pawn|GetController _aspawn)))) (Utilities|Name|MakeLiteralName "is Stanned?"))) (not (Variables|/Game/Blueprints/BP_Cultist_Parent.BP_Cultist_Parent_C|GetProtected_By_Mask? _asbp_cultist_parent))))
    (else
      (bind _asbp_parasite_2 (Utilities|Casting|CastToBP_Parasite (Pawn|GetControlledPawn)))
      (Sprite|SetFlipbook (Variables|/Game/Blueprints/BP_Characters_Parent.BP_Characters_Parent_C|GetGun_FlipBook _asbp_parasite_2) "/Game/Flipbooks/FB_Tentacle_Idle.FB_Tentacle_Idle")
      (return 0 (Math|Boolean|ANDBoolean (> (Math|Vector|DotProduct (Math|Vector|Normalize (- (Transformation|GetActorLocation _aspawn) (Transformation|GetActorLocation (Pawn|GetControlledPawn)))) (Math|Vector|GetForwardVector (Variables|/Script/Engine.Actor|GetRootComponent _aspawn))) 0.1) (not (ScalableFloat|GetValueasBool (AI|GetBlackboard (.AsBP%20Enemy%20Controller (Utilities|Casting|CastToBP_Enemy_Controller (Pawn|GetController _aspawn)))) (Utilities|Name|MakeLiteralName "is Stanned?"))) (not (Variables|/Game/Blueprints/BP_Cultist_Parent.BP_Cultist_Parent_C|GetProtected_By_Mask? _asbp_cultist_parent)))))))