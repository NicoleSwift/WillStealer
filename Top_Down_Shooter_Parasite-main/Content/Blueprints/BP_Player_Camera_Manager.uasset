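; Player camera manager that drives a smoothed, angled top-down camera for BP_Characters_Parent view targets.
; BlueprintUpdateCamera pushes a focus point out from the character's ArrowGun along its forward vector by a quarter of the flat pawn-to-cursor-hit distance.
; VInterpTo eases the stored position toward that point, then adds a fixed offset, rotation and FOV.
; An alternative Focused-based position selection is left unconnected.
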(event EventBeginPlay)

(event Collision|EventActorBeginOverlap
  (params (OtherActor :type Actor%20Object%20Reference)))

(event EventTick
  (params (DeltaSeconds :type Float%20%28single-precision%29)))

(fn ConstructionScript)

(fn BlueprintUpdateCamera
  (params (CameraTarget :type Actor%20Object%20Reference))
  (bind _returnvalue (Game|GetPlayerController 0))
  (bind _returnvalue_2 (Game|Player|GetPlayerPawn 0))
  (bind _hitresult (Game|Player|GetHitResultUnderCursorbyChannel _returnvalue "TraceTypeQuery3" true))
  (bind _returnvalue_3 (Transformation|GetActorLocation _returnvalue_2))
  (bind _location (Collision|BreakHitResult _hitresult))
  (bind _asbp_characters_parent (Utilities|Casting|CastToBP_Characters_Parent CameraTarget))
  (bind _output_get (Variables|Default|SetPrev_Camera_Position (Math|Interpolation|VInterpTo (Variables|Default|GetPrev_Camera_Position) (+ (Transformation|GetWorldLocation (Variables|/Game/Blueprints/BP_Characters_Parent.BP_Characters_Parent_C|GetArrow_Gun _asbp_characters_parent)) (* (Math|Vector|GetForwardVector (Variables|/Game/Blueprints/BP_Characters_Parent.BP_Characters_Parent_C|GetArrow_Gun _asbp_characters_parent)) (* (Math|Vector|Distance(Vector) (Math|Vector|MakeVector (.x _returnvalue_3) (.y _returnvalue_3) 0.0) (Math|Vector|MakeVector (.x _location) (.y _location) 0.0)) 0.25))) (Utilities|Time|GetWorldDeltaSeconds) 5.0)))
  (return (+ _output_get (Math|Vector|MakeVector 0.0 125.0 3e+02)) (Math|Rotator|MakeRotator 0.0 (+ 2.7e+02 3e+01) (+ -9e+01 0.0)) 9e+01 true))